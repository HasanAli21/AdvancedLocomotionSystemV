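; Parent Blueprint for an obstacle that moves along world X or Y while a tagged player is in its Box trigger.
; BeginPlay turns the Forward, Backward, Right or Left flag and Speed into a velocity.
; Tick applies it, scaled by delta time, through MoveFunctionality without sweeping, printing the direction for debugging.
; Leaving the box stops movement unless IsInfinit is set, which keeps it moving once triggered.
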(event `self.ReceiveBeginPlay`
  (bind _speed (`self.Speed`))
  (bind _returnvalue (* _speed -1.0))
  (`|ExecutionSequence`
    (:`then_0`
      (if (`self.Forward?`)
        (set `self.MovementSpeed` (`KismetMathLibrary.MakeVector` _speed))))
    (:`then_1`
      (if (`self.Backward?`)
        (set `self.MovementSpeed` (`KismetMathLibrary.MakeVector` _returnvalue))))
    (:`then_2`
      (if (`self.Right?`)
        (set `self.MovementSpeed` (`KismetMathLibrary.MakeVector` 0.0 _speed))))
    (:`then_3`
      (if (`self.Left?`)
        (set `self.MovementSpeed` (`KismetMathLibrary.MakeVector` 0.0 _returnvalue))))))

(event `self.ReceiveTick`
  (params (DeltaSeconds :type "Float (single-precision)"))
  (set `self.DeltaTime` DeltaSeconds)
  (if (`self.IsPlayerOn`)
    (`|ExecutionSequence`
      (:`then_0`
        (if (`self.Forward?`)
          (`self.MoveFunctionality` (`self.MovementSpeed`))
          (`KismetSystemLibrary.PrintString` "Forward")))
      (:`then_1`
        (if (`self.Backward?`)
          (`self.MoveFunctionality` (`self.MovementSpeed`))
          (`KismetSystemLibrary.PrintString` "Backward")))
      (:`then_2`
        (if (`self.Right?`)
          (`self.MoveFunctionality` (`self.MovementSpeed`))
          (`KismetSystemLibrary.PrintString` "Right")))
      (:`then_3`
        (if (`self.Left?`)
          (`self.MoveFunctionality` (`self.MovementSpeed`))
          (`KismetSystemLibrary.PrintString` "Left"))))))

(event `self.Box.OnComponentBeginOverlap`
  (params (OverlappedComponent :type "PrimitiveComponent Object Reference") (OtherActor :type "Actor Object Reference") (OtherComp :type "PrimitiveComponent Object Reference") (OtherBodyIndex :type Integer) (bFromSweep :type Boolean) (SweepResult :type "HitResult Structure (by ref)"))
  (if (`self.ActorHasTag` OtherActor (`self.PlayerTag`))
    (set `self.IsPlayerOn` true)))

(event `self.Box.OnComponentEndOverlap`
  (params (OverlappedComponent :type "PrimitiveComponent Object Reference") (OtherActor :type "Actor Object Reference") (OtherComp :type "PrimitiveComponent Object Reference") (OtherBodyIndex :type Integer))
  (if (`self.ActorHasTag` OtherActor (`self.PlayerTag`))
    (if (not (`self.IsInfinit`))
      (set `self.IsPlayerOn` false))))

(fn `MoveFunctionality`
  (params (MoveSpeed :type "Vector Structure"))
  (`self.K2_SetActorLocation` (+ (* MoveSpeed (`self.DeltaTime`)) (`self.K2_GetActorLocation`))))

(fn `UserConstructionScript`)