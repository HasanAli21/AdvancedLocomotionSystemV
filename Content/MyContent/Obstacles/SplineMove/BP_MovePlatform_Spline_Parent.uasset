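; Parent Blueprint for a platform obstacle that shuttles back and forth along a spline, pausing at each end before reversing.
; Tick advances a clamped time, and UpdateLocation remaps it through a float curve to place the mesh.
; Movement runs once enabled by a construction-time flag or player overlap.
; An optional hold mode delays movement through a retriggerable delay refreshed while the player overlaps.
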(event `self.ReceiveTick`
  (params (DeltaSeconds :type "Float (single-precision)"))
  (bind _movementtime (`self.MovementTime`))
  (`|ExecutionSequence`
    (:`then_0`
      (`self.HoldFunctinolaity` (`self.DurationTime`)
        (:`Output`
          (set `self.DeltaSeconds` DeltaSeconds :!label _label)
          (if (`self.MoveWithJustCollide`)
            (if (`self.CanMove?`)
              (set `self.MovementTime` (`KismetMathLibrary.FClamp` (+ (`self.MovementTime`) (* (`self.MovementDirection`) (`self.DeltaSeconds`))) 0.0 (`SplineComponent.Duration` (`self.Spline`))))
              (`/Engine/EditorBlueprintResources/StandardMacros.CompareInt` (`self.MovementDirection`)
                (:`>`
                  (if (`KismetMathLibrary.NearlyEqual_FloatFloat` (`SplineComponent.Duration` (`self.Spline`)) _movementtime)
                    (set `self.CanMove?` false :!label _label_2)
                    (set `self.MovementDirection` (* (`self.MovementDirection`) -1))
                    (`KismetSystemLibrary.Delay` (`self.MovementDelay`))
                    (set `self.CanMove?` true)
                    (else
                      (`self.UpdateLocation` :!label _label_3))))
                (:`<`
                  (if (`KismetMathLibrary.NearlyEqual_FloatFloat` _movementtime)
                    (goto _label_2)
                    (else
                      (goto _label_3))))))))))
    (:`then_1`
      (if (`self.DurationDone?`)
        (goto _label)))))

(event `self.Collision.OnComponentBeginOverlap`
  (params (OverlappedComponent :type "PrimitiveComponent Object Reference") (OtherActor :type "Actor Object Reference") (OtherComp :type "PrimitiveComponent Object Reference") (OtherBodyIndex :type Integer) (bFromSweep :type Boolean) (SweepResult :type "HitResult Structure (by ref)"))
  (if (`self.ActorHasTag` OtherActor "Player")
    (set `self.IsPlayerCollide?` true)
    (set `self.MoveWithJustCollide` true)))

(event `self.Collision.OnComponentEndOverlap`
  (params (OverlappedComponent :type "PrimitiveComponent Object Reference") (OtherActor :type "Actor Object Reference") (OtherComp :type "PrimitiveComponent Object Reference") (OtherBodyIndex :type Integer))
  (if (`self.ActorHasTag` OtherActor "Player")
    (set `self.IsPlayerCollide?` false)))

(fn `UpdateLocation`
  (bind _duration (`SplineComponent.Duration` (`self.Spline`)))
  (`SceneComponent.K2_SetWorldLocation` (`self.StaticMesh`) (`SplineComponent.GetLocationAtTime` (`self.Spline`) (`KismetMathLibrary.MapRangeClamped` (`CurveFloat.GetFloatValue` (`self.MovementCurve`) (`KismetMathLibrary.NormalizeToRange` (`self.MovementTime`) 0.0 _duration)) 0.0 1.0 0.0 _duration) "World" false) false false))

(fn `UserConstructionScript`
  (set `self.MoveWithJustCollide` (`self.StartWithPlayer`))
  (set `SplineComponent.Duration` (`self.MovementDuration`) (`self.Spline`))
  (set `self.MovementTime` (* (`self.StartPosition`) (`self.MovementDuration`)))
  (`self.UpdateLocation`))