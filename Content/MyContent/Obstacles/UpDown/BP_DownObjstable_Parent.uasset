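; Parent obstacle actor that moves up or down while the player is on it.
; Box overlaps with actors carrying the player tag set a flag that lets Tick move the actor by DownSpeed, scaled by delta time and a sign chosen from IsUp at BeginPlay.
; When IsInfinit is set, the end overlap leaves the flag on, so movement continues indefinitely once triggered.
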(event `self.ReceiveBeginPlay`
  (if (`self.IsUp?`)
    (set `self.UpDown?` 1.0)
    (else
      (set `self.UpDown?` -1.0))))

(event `self.ReceiveTick`
  (params (DeltaSeconds :type "Float (single-precision)"))
  (if (`self.IsInfinit`)
    (`self.MoveDownFunctionality` DeltaSeconds)
    (else
      (`self.MoveDownFunctionality` DeltaSeconds))))

(event `self.Box.OnComponentBeginOverlap`
  (params (OverlappedComponent :type "PrimitiveComponent Object Reference") (OtherActor :type "Actor Object Reference") (OtherComp :type "PrimitiveComponent Object Reference") (OtherBodyIndex :type Integer) (bFromSweep :type Boolean) (SweepResult :type "HitResult Structure (by ref)"))
  (if (`self.ActorHasTag` OtherActor (`self.PlayerTag`))
    (set `self.IsPlayerOn` true)))

(event `self.Box.OnComponentEndOverlap`
  (params (OverlappedComponent :type "PrimitiveComponent Object Reference") (OtherActor :type "Actor Object Reference") (OtherComp :type "PrimitiveComponent Object Reference") (OtherBodyIndex :type Integer))
  (if (`self.ActorHasTag` OtherActor (`self.PlayerTag`))
    (if (not (`self.IsInfinit`))
      (set `self.IsPlayerOn` false))))

(fn `MoveDownFunctionality`
  (params (InputPin :type "Float (single-precision)"))
  (if (`self.IsPlayerOn`)
    (`self.K2_SetActorLocation` (+ (`self.K2_GetActorLocation`) (* InputPin (`self.DownSpeed`) (`self.UpDown?`))))))

(fn `UserConstructionScript`)